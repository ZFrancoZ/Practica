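; Elevator Blueprint (Asensor) that raises its platform once no collectable targets remain in the level.
; On Box begin overlap by any actor, it checks CollectableLeftTargets on FirstPersonGameMode and, at zero, plays a timeline.
; The timeline track, scaled by a fixed travel height, drives the Asensor component's relative Z.
; When a FirstPersonCharacter leaves the box, the timeline reverses and lowers it.
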(event OnComponentBeginOverlap(Box)
  (params (OverlappedComponent :type Primitive%20Component%20Object%20Reference) (OtherActor :type Actor%20Object%20Reference) (OtherComp :type Primitive%20Component%20Object%20Reference) (OtherBodyIndex :type Integer) (bFromSweep :type Boolean) (SweepResult :type Hit%20Result%20Structure%20%28by%20ref%29))
  (bind _asfirst_person_game_mode (Utilities|Casting|CastToFirstPersonGameMode (Game|GetGameMode)))
  (if (== (Variables|/Game/FirstPersonBP/Blueprints/FirstPersonGameMode.FirstPersonGameMode_C|GetCollectable%20Left%20%28Targets%29 _asfirst_person_game_mode) 0)
    (bind _newtrack_0 (Timeline|Timeline_0 Play)
      (:Update
        (Transformation|SetRelativeLocation (Variables|Default|GetAsensor) (Math|Vector|MakeVector 0.0 0.0 (* _newtrack_0 1.3e+03)) false false)))))

(event OnComponentEndOverlap(Box)
  (params (OverlappedComponent :type Primitive%20Component%20Object%20Reference) (OtherActor :type Actor%20Object%20Reference) (OtherComp :type Primitive%20Component%20Object%20Reference) (OtherBodyIndex :type Integer))
  (Utilities|Casting|CastToFirstPersonCharacter OtherActor)
  (bind _newtrack_0 (Timeline|Timeline_0 Reverse)
    (:Update
      (Transformation|SetRelativeLocation (Variables|Default|GetAsensor) (Math|Vector|MakeVector 0.0 0.0 (* _newtrack_0 1.3e+03)) false false))))

(fn ConstructionScript)