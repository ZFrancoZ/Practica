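; Enemigo is an enemy Blueprint that acts as a game-ending trigger when the FirstPersonCharacter overlaps its Box.
; The overlap enlarges LargeMesh, calls DisableInput, then after a short delay plays a timeline that drives the mesh along its relative X axis.
; The end sequence hangs off the timeline's Update rather than Finished, using delays to show Widget_End and then quit the game.
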(event OnComponentBeginOverlap(Box)
  (params (OverlappedComponent :type Primitive%20Component%20Object%20Reference) (OtherActor :type Actor%20Object%20Reference) (OtherComp :type Primitive%20Component%20Object%20Reference) (OtherBodyIndex :type Integer) (bFromSweep :type Boolean) (SweepResult :type Hit%20Result%20Structure%20%28by%20ref%29))
  (bind _asfirst_person_character (Utilities|Casting|CastToFirstPersonCharacter OtherActor))
  (Transformation|SetRelativeScale3D (Variables|Default|GetLarge_Mesh) "1.400000,1.400000,1.400000")
  (Input|DisableInput (Game|GetGameMode) 0)
  (Utilities|FlowControl|Delay 1.0)
  (bind _newtrack_0 (Timeline|Timeline_1 Play)
    (:Update
      (Transformation|SetRelativeLocation (Variables|Default|GetLarge_Mesh) (Math|Vector|MakeVector (* _newtrack_0 1.5e+03) 0.0 0.0) false false)
      (Utilities|FlowControl|Delay 0.2)
      (bind _returnvalue (UserInterface|CreateWidget "/Game/Blueprints/Widget_End.Widget_End_C"))
      (UserInterface|Viewport|AddtoViewport _returnvalue 0)
      (Utilities|FlowControl|Delay 3.0)
      (Game|QuitGame 0 "Quit" false))))

(fn ConstructionScript)