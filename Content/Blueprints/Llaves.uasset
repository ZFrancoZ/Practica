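; Llaves ("keys") is a collectable actor that the player collects by shooting it, with a constantly spinning Jarron component.
; When a FirstPersonProjectile hits its Box, it decrements the remaining keys counter on FirstPersonGameMode, adds a new Widget_Llaves to the viewport and destroys itself.
; Tick applies the yaw spin scaled by delta time, so rotation speed is frame-rate independent.
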(event OnComponentHit(Box)
  (params (HitComponent :type Primitive%20Component%20Object%20Reference) (OtherActor :type Actor%20Object%20Reference) (OtherComp :type Primitive%20Component%20Object%20Reference) (NormalImpulse :type Vector :default "0, 0, 0") (Hit :type Hit%20Result%20Structure%20%28by%20ref%29))
  (Utilities|Casting|CastToFirstPersonProjectile OtherActor)
  (bind _asfirst_person_game_mode (Utilities|Casting|CastToFirstPersonGameMode (Game|GetGameMode)))
  (bind _result (Math|Integer|DecrementInt (Variables|/Game/FirstPersonBP/Blueprints/FirstPersonGameMode.FirstPersonGameMode_C|GetCollectable%20left%20%28Llaves%29 _asfirst_person_game_mode))
    (:%20%20
      (Variables|/Game/FirstPersonBP/Blueprints/FirstPersonGameMode.FirstPersonGameMode_C|SetCollectable%20left%20%28Llaves%29 _asfirst_person_game_mode _result)
      (bind _returnvalue (UserInterface|CreateWidget "/Game/Blueprints/Widget_LLaves.Widget_Llaves_C"))
      (UserInterface|Viewport|AddtoViewport _returnvalue 0)
      (Actor|DestroyActor))))

(event EventTick
  (params (DeltaSeconds :type Float%20%28single-precision%29))
  ;[1 1 1] Rotacion Constante
  (Transformation|AddRelativeRotation (Variables|Default|GetJarron) (Math|Rotator|MakeRotator 0.0 0.0 (* DeltaSeconds 4e+01)) false false))

(fn ConstructionScript)