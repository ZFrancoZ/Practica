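; Final door actor that slides open once the game mode's key counter (CollectableLeftLlaves) matches its SeActivo value.
; Any overlap on Box runs that check, then sets SeActivo to 5 and plays DoorTimer, a timeline moving Puerta along its relative Y axis.
; A FirstPersonCharacter overlapping Box2 reverses the timeline to slide the door back.
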(event OnComponentBeginOverlap(Box2)
  (params (OverlappedComponent :type Primitive%20Component%20Object%20Reference) (OtherActor :type Actor%20Object%20Reference) (OtherComp :type Primitive%20Component%20Object%20Reference) (OtherBodyIndex :type Integer) (bFromSweep :type Boolean) (SweepResult :type Hit%20Result%20Structure%20%28by%20ref%29))
  (Utilities|Casting|CastToFirstPersonCharacter OtherActor)
  (bind _newtrack_0 (Timeline|DoorTimer Reverse)
    (:Update
      (Transformation|SetRelativeLocation (Variables|Default|GetPuerta) (Math|Vector|MakeVector 0.0 (* _newtrack_0 1.5e+02) 0.0) false false))))

(event OnComponentBeginOverlap(Box)
  (params (OverlappedComponent :type Primitive%20Component%20Object%20Reference) (OtherActor :type Actor%20Object%20Reference) (OtherComp :type Primitive%20Component%20Object%20Reference) (OtherBodyIndex :type Integer) (bFromSweep :type Boolean) (SweepResult :type Hit%20Result%20Structure%20%28by%20ref%29))
  (bind _asfirst_person_game_mode (Utilities|Casting|CastToFirstPersonGameMode (Game|GetGameMode)))
  (if (== (Variables|/Game/FirstPersonBP/Blueprints/FirstPersonGameMode.FirstPersonGameMode_C|GetCollectable%20left%20%28Llaves%29 _asfirst_person_game_mode) (Variables|Default|GetSe%20activo))
    (Variables|Default|SetSe%20activo 5)
    (bind _newtrack_0 (Timeline|DoorTimer Play)
      (:Update
        (Transformation|SetRelativeLocation (Variables|Default|GetPuerta) (Math|Vector|MakeVector 0.0 (* _newtrack_0 1.5e+02) 0.0) false false)))))

(fn ConstructionScript)